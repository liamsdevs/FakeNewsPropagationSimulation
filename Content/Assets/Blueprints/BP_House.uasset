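; BP_House is a house actor that spawns and tracks its BP_Agent inhabitants.
; SpawnAgents clears AgentsRef, spawns one agent per AgentsInfos entry with those attributes and itself as House, then stores each reference.
; Spawns sit at a fixed height around the Cube; X and Y use separate random angles scaled by the Sphere radius, so they scatter within a square rather than on the circle.
; Event graph and construction script are empty, so SpawnAgents relies on an external call.
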(fn `SpawnAgents`
  (bind _returnvalue (`KismetMathLibrary.RandomFloatInRange` 0.0 359.0))
  (bind (_returnvalue_x _returnvalue_y) (`KismetMathLibrary.BreakVector` (`SceneComponent.K2_GetComponentLocation` (`self.Cube`))))
  (bind _sphereradius (`SphereComponent.SphereRadius` (`self.Sphere`)))
  (`KismetArrayLibrary.Array_Clear` (`self.AgentsRef`))
  (for _array_element (`self.AgentsInfos`)
    (bind _returnvalue_2 (`|SpawnActorFromClass` "/Game/Assets/Blueprints/AI/BP_Agent.BP_Agent_C" (`KismetMathLibrary.MakeTransform` (`KismetMathLibrary.MakeVector` (+ _returnvalue_x (* (`KismetMathLibrary.DegCos` _returnvalue) _sphereradius)) (+ _returnvalue_y (* (`KismetMathLibrary.DegSin` _returnvalue) _sphereradius)) 100.0)) "AlwaysSpawn" "MultiplyWithRoot" null _array_element self null))
    (`KismetArrayLibrary.Array_Add` (`self.AgentsRef`) _returnvalue_2)))

(fn `UserConstructionScript`)