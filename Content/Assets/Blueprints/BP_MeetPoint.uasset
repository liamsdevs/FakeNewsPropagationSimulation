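; BP_MeetPoint is a meeting point that simulates belief spreading among BP_Agent actors as Ignorant, Sceptique or Croyant states.
; UpdateStateOfAgents gathers agents overlapping its Sphere and buckets them by state through FilterAgents.
; Three sequential rules re-count live states: believers randomly convert the ignorant, enough sceptics fact-check believers, and a believer majority threshold resets sceptics to ignorant.
; It finally flags the meeting as done on each agent's AI controller.
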(fn `FilterAgents`
  (params (Agents :type "Array of /Game/Assets/Blueprints/AI/BP_Agent Object Reference"))
  (returns (Croyants :type "Array of /Game/Assets/Blueprints/AI/BP_Agent Object Reference") (Sceptiques :type "Array of /Game/Assets/Blueprints/AI/BP_Agent Object Reference") (Ignorants :type "Array of /Game/Assets/Blueprints/AI/BP_Agent Object Reference"))
  (locals (Croyant :type "Array of /Game/Assets/Blueprints/AI/BP_Agent Object Reference") (Sceptique :type "Array of /Game/Assets/Blueprints/AI/BP_Agent Object Reference") (Ignorant :type "Array of /Game/Assets/Blueprints/AI/BP_Agent Object Reference"))
  (`KismetArrayLibrary.Array_Clear` (`local.Sceptique`))
  (`KismetArrayLibrary.Array_Clear` (`local.Croyant`))
  (`KismetArrayLibrary.Array_Clear` (`local.Ignorant`))
  (for _array_element Agents
    (bind (_attributes_persuasionpower _attributes_timebeforedoubt _attributes_state) (break `/Game/Assets/Blueprints/S_AgentAttributes` (`/Game/Assets/Blueprints/AI/BP_Agent.Attributes` _array_element)))
    (`KismetArrayLibrary.Array_Add` (select `/Game/Assets/Blueprints/E_AgentState` _attributes_state :`NewEnumerator0` (`local.Ignorant`) :`NewEnumerator1` (`local.Sceptique`) :`NewEnumerator2` (`local.Croyant`)) _array_element))
  (return (`local.Croyant`) (`local.Sceptique`) (`local.Ignorant`)))

(fn `GetAllAgentsInside`
  (returns (OverlappingAgents :type "Array of /Game/Assets/Blueprints/AI/BP_Agent Object Reference"))
  (locals (Agents :type "Array of /Game/Assets/Blueprints/AI/BP_Agent Object Reference"))
  (`KismetArrayLibrary.Array_Clear` (`local.Agents`))
  (for _array_element (`PrimitiveComponent.GetOverlappingActors` (`self.Sphere`) "/Game/Assets/Blueprints/AI/BP_Agent.BP_Agent_C")
    (bind _asbp_agent (cast `/Game/Assets/Blueprints/AI/BP_Agent` _array_element))
    (`KismetArrayLibrary.Array_Add` (`local.Agents`) _asbp_agent))
  (return (`local.Agents`)))

(fn `UpdateStateOfAgents`
  (locals (AgentsInMeetingPoint :type "Array of /Game/Assets/Blueprints/AI/BP_Agent Object Reference"))
  (bind _overlappingagents (`self.GetAllAgentsInside`))
  (bind _returnvalue (`KismetMathLibrary.RandomFloatInRange` 0.0 1.0))
  (bind (_croyants _sceptiques) (`self.FilterAgents` _overlappingagents))
  (bind _returnvalue_2 (`KismetArrayLibrary.Array_Length` _croyants))
  (set `local.AgentsInMeetingPoint` _overlappingagents)
  ;[1 1 1] Regle 1 Propagation
  (if (> _returnvalue_2 0)
    (for _array_element (`local.AgentsInMeetingPoint`)
      (if (`|EnumEquality` (`/Game/Assets/Blueprints/AI/BP_Agent.GetState` _array_element) "NewEnumerator0")
        (if (< _returnvalue (`KismetMathLibrary.FClamp` (* _returnvalue_2 0.2)))
          (`/Game/Assets/Blueprints/AI/BP_Agent.UpdateState` _array_element (select `bool` (< _returnvalue 0.15) :`false` "NewEnumerator2" :`true` "NewEnumerator1" :!type "/Game/Assets/Blueprints/E_AgentState Enum"))))))
  ;[1 1 1] Regle 2 : FactChecking
  (if (>= (`KismetArrayLibrary.Array_Length` _sceptiques) 3)
    (for _array_element_2 (`local.AgentsInMeetingPoint`)
      (if (`|EnumEquality` (`/Game/Assets/Blueprints/AI/BP_Agent.GetState` _array_element_2) "NewEnumerator2")
        (if (< (`KismetMathLibrary.RandomFloatInRange` 0.0 1.0) 0.3)
          (`/Game/Assets/Blueprints/AI/BP_Agent.UpdateState` _array_element_2 (select `bool` (`KismetMathLibrary.RandomBool`) :`false` "NewEnumerator1" :`true` "NewEnumerator0" :!type "/Game/Assets/Blueprints/E_AgentState Enum"))))))
  ;[1 1 1] Regle 3
  (if (>= _returnvalue_2 5)
    (for _array_element_3 (`local.AgentsInMeetingPoint`)
      (if (`|EnumEquality` (`/Game/Assets/Blueprints/AI/BP_Agent.GetState` _array_element_3) "NewEnumerator1")
        (`/Game/Assets/Blueprints/AI/BP_Agent.UpdateState` _array_element_3 "NewEnumerator0"))))
  (for _array_element_4 (`local.AgentsInMeetingPoint`)
    (`/Game/Assets/Blueprints/AI/BP_AIController.SetMeetingDone` (`/Game/Assets/Blueprints/AI/BP_Agent.As BP AIController` _array_element_4) true)))

(fn `UserConstructionScript`)