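; RTS camera pawn that pans, rotates and zooms through a spring arm.
; Axis inputs and cursor checks at the viewport edges feed movement input along the actor's forward and right vectors.
; Yaw turns the actor via a rotation axis or mouse while a button is held, which also tilts the arm within clamped pitch.
; Zoom clamps a target arm length and interpolates toward it, starting at a third of maximum.
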(event `self.ReceiveBeginPlay`
  (`|ExecutionSequence`
    (:`then_1`
      (bind _output_get (set `SpringArmComponent.TargetArmLength` (/ (`self.MaxZoom`) 3.0) (`self.SpringArm`)))
      (set `self.NewTargetArmLength` _output_get))))

(event `InputAction|MouseRotationActivate`
  (params (Key :type "Key Structure"))
  (:`Pressed`
    (set `self.MouseActivateRotation` true))
  (:`Released`
    (set `self.MouseActivateRotation` false)))

(event `InputAxis|MoveForward`
  (params (AxisValue :type "Float (single-precision)"))
  (`self.MoveForward` AxisValue))

(event `InputAxis|MoveRight`
  (params (AxisValue :type "Float (single-precision)"))
  (`self.MoveRight` AxisValue))

(event `InputAxis|RotateRTSCam`
  (params (AxisValue :type "Float (single-precision)"))
  (`self.RotateCamera` AxisValue))

(event `InputAxis|ZoomRTSCam`
  (params (AxisValue :type "Float (single-precision)"))
  (`self.Zoom` AxisValue))

(event `InputAxis|MouseRotateUp`
  (params (AxisValue :type "Float (single-precision)"))
  (if (`self.MouseActivateRotation`)
    (`self.RotateCameraUp` AxisValue)))

(event `InputAxisKey|MouseX`
  (params (AxisValue :type "Float (single-precision)"))
  (bind (_returnvalue_x _returnvalue_y) (`KismetMathLibrary.BreakVector2D` (`WidgetLayoutLibrary.GetViewportSize`)))
  (bind _returnvalue (/ (`.LocationY` (`PlayerController.GetMousePosition` (`GameplayStatics.GetPlayerController` 0))) _returnvalue_y))
  (if (> _returnvalue 0.98)
    (`self.MoveForward` -1.0)
    (elif (< _returnvalue 0.02)
      (`self.MoveForward` 1.0))))

(event `InputAxis|MouseRotate`
  (params (AxisValue :type "Float (single-precision)"))
  (if (`self.MouseActivateRotation`)
    (`self.RotateCamera` AxisValue)))

(event `InputAxisKey|MouseY`
  (params (AxisValue :type "Float (single-precision)"))
  (bind (_returnvalue_x _returnvalue_y) (`KismetMathLibrary.BreakVector2D` (`WidgetLayoutLibrary.GetViewportSize`)))
  (bind _returnvalue (/ (`PlayerController.GetMousePosition` (`GameplayStatics.GetPlayerController` 0)) _returnvalue_x))
  (if (> _returnvalue 0.98)
    (`self.MoveRight` 1.0)
    (elif (< _returnvalue 0.02)
      (`self.MoveRight` -1.0))))

(fn `MoveForward`
  (params (AxisValue :type "Float (double-precision)"))
  (`self.AddMovementInput` (`self.GetActorForwardVector`) (* AxisValue (`self.MovementSpeed`))))

(fn `MoveRight`
  (params (AxisValue :type "Float (double-precision)"))
  (`self.AddMovementInput` (`self.GetActorRightVector`) (* AxisValue (`self.MovementSpeed`))))

(fn `RotateCamera`
  (params (AxisValue :type "Float (double-precision)"))
  (bind (_returnvalue_roll _returnvalue_pitch _returnvalue_yaw) (`KismetMathLibrary.BreakRotator` (`self.K2_GetActorRotation`)))
  (`self.K2_SetActorRotation` (`KismetMathLibrary.MakeRotator` _returnvalue_roll _returnvalue_pitch (`KismetMathLibrary.FClamp` (+ _returnvalue_yaw (* AxisValue (`self.CameraRotationSpeed`))) -360.0 360.0))))

(fn `RotateCameraUp`
  (params (AxisValue :type "Float (double-precision)"))
  (bind _springarm (`self.SpringArm`))
  (bind (_returnvalue_roll _returnvalue_pitch _returnvalue_yaw) (`KismetMathLibrary.BreakRotator` (`SpringArmComponent.GetTargetRotation` _springarm)))
  (`SceneComponent.K2_SetWorldRotation` _springarm (`KismetMathLibrary.MakeRotator` 0.0 (`KismetMathLibrary.FClamp` (+ (* AxisValue (`self.CameraRotationSpeed`)) _returnvalue_pitch) -80.0 -10.0) _returnvalue_yaw) false false))

(fn `UserConstructionScript`)

(fn `Zoom`
  (params (AxisValue :type "Float (double-precision)"))
  (bind _springarm (`self.SpringArm`))
  (bind _output_get (set `self.NewTargetArmLength` (`KismetMathLibrary.FClamp` (+ (* AxisValue (`self.ZoomSpeed`)) (`self.NewTargetArmLength`)) (`self.MinZoom`) (`self.MaxZoom`))))
  (set `SpringArmComponent.TargetArmLength` (`KismetMathLibrary.FInterpTo` (`SpringArmComponent.TargetArmLength` _springarm) _output_get (`GameplayStatics.GetWorldDeltaSeconds`) 15.0) _springarm))