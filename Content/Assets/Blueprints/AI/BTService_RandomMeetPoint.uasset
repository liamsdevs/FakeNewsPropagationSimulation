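; Behavior tree service that, on activation, writes a meet point location to a blackboard key for the controlled AI pawn.
; It caches the simulation manager game mode, printing an error if the cast fails, and takes the location of a random actor from its meet point list.
; A validity-based select offers a random reachable point near the pawn as fallback, though that path runs only with a manager set.
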(event `self.ReceiveActivationAI`
  (params (OwnerController :type "AIController Object Reference") (ControlledPawn :type "Pawn Object Reference"))
  (bind _as_gm_simulation_manger (`self.As GM Simulation Manger`))
  (`/Engine/EditorBlueprintResources/StandardMacros.IsValid` (`self.As GM Simulation Manger`)
    (:`Is Valid`
      (`BTFunctionLibrary.SetBlackboardValueAsVector` (`self.BlackboardKey`) (`KismetMathLibrary.SelectVector` (`Actor.K2_GetActorLocation` (`KismetArrayLibrary.Array_Random` (`/Game/Assets/Core/GM_SimulationManager.MeetPointsRef` _as_gm_simulation_manger))) (`NavigationSystemV1.K2_GetRandomReachablePointInRadius` (`Actor.K2_GetActorLocation` ControlledPawn) 500.0 null null) (`KismetSystemLibrary.IsValid` _as_gm_simulation_manger)) :!label _label))
    (:`Is Not Valid`
      (bind _asgm_simulation_manger (cast `/Game/Assets/Core/GM_SimulationManager` (`GameplayStatics.GetGameMode`))
        (:`then`
          (set `self.As GM Simulation Manger` _asgm_simulation_manger)
          (goto _label))
        (:`CastFailed`
          (`KismetSystemLibrary.PrintString` "Error : AI Service RandomMeetPoint Casting to Gamemode"))))))