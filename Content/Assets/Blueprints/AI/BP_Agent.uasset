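; BP_Agent is an AI agent with a belief state (Ignorant, Sceptique or Croyant), shown through the material on its cylinder.
; UpdateState writes the state into the Attributes struct, alongside persuasion power and doubt time, and swaps the material; the construction script applies it.
; On BeginPlay, the agent writes its House location to the BP_AIController blackboard as HouseLocation.
; TryToConvince is an empty stub, and GetState exposes the current state.
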(event `self.ReceiveBeginPlay`
  (bind _asbp_aicontroller (cast `/Game/Assets/Blueprints/AI/BP_AIController` (`AIBlueprintHelperLibrary.GetAIController` self)))
  (bind _output_get (set `self.As BP AIController` _asbp_aicontroller))
  (`BlackboardComponent.SetValueAsVector` (`AIController.Blackboard` _output_get) "HouseLocation" (`self.K2_GetActorLocation` (`self.House`))))

(fn `GetState`
  (returns (State :type "/Game/Assets/Blueprints/E_AgentState Enum"))
  (return (`.State_7_3731AFB7487352857FD96DB02C120604` (break `/Game/Assets/Blueprints/S_AgentAttributes` (`self.Attributes`)))))

(fn `TryToConvince`
  (params (otherAgent :type "/Game/Assets/Blueprints/AI/BP_Agent Object Reference")))

(fn `UpdateState`
  (params (State :type "/Game/Assets/Blueprints/E_AgentState Enum" :default "NewEnumerator0"))
  (bind (_attributes_persuasionpower _attributes_timebeforedoubt) (break `/Game/Assets/Blueprints/S_AgentAttributes` (`self.Attributes`)))
  (set `self.Attributes` (make `/Game/Assets/Blueprints/S_AgentAttributes` _attributes_persuasionpower _attributes_timebeforedoubt State))
  (`PrimitiveComponent.SetMaterial` (`self.Cylinder`) 0 (select `/Game/Assets/Blueprints/E_AgentState` State :`NewEnumerator0` (`self.IgnorantMaterial`) :`NewEnumerator1` (`self.SceptiqueMaterial`) :`NewEnumerator2` (`self.CroyantMaterial`) :!type "MaterialInterface Object Reference")))

(fn `UserConstructionScript`
  (`self.UpdateState` (`.State_7_3731AFB7487352857FD96DB02C120604` (break `/Game/Assets/Blueprints/S_AgentAttributes` (`self.Attributes`)))))