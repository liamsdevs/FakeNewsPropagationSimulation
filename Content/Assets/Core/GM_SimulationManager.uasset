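; Game mode that runs a generation-based simulation of agents whose states are Ignorant, Sceptique or Croyant, from setup menu to results.
; StartSimulation has the WorldManager place meet points and houses, sized at three agents each, then spawns agents.
; One-second timers poll AI readiness, alternating meetings that update agent states with returns home that begin the next generation.
; State counts per generation feed the HUD and, once StopSimulation is set, the result screen.
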(event `self.ReceiveBeginPlay`
  (bind _returnvalue (`GameplayStatics.GetActorOfClass` "/Game/Assets/Core/BP_WorldManager.BP_WorldManager_C"))
  (bind _output_get (set `self.WorldManager` _returnvalue))
  (`/Engine/EditorBlueprintResources/StandardMacros.IsValid` _output_get
    (:`Is Valid`
      (`self.ShowMenu`))
    (:`Is Not Valid`
      (`KismetSystemLibrary.PrintString` "Error : No World Manager"))))

(event `StartSimulation`
  (params (SimulationSettings :type "/Game/Assets/Blueprints/S_SimulationSettings Structure"))
  (bind (_numberofagents _numberofmeetpoint) (break `/Game/Assets/Blueprints/S_SimulationSettings` SimulationSettings))
  (bind (_sceptiquesn _croyantsn _ignorantsn) (`self.CalculateNumbersOfAgentsPerTypes`))
  (bind _generation (`self.Generation`))
  (bind _whud (`self.WHud`))
  (`BlueprintMapLibrary.Map_Clear` (`self.Infos`))
  (set `self.NumOfAgents` _numberofagents)
  (set `self.NumOfMeetPoints` _numberofmeetpoint)
  (set `self.Generation` 1)
  (bind _output_get (set `self.NumOfHouses` (`self.DetermineNumberOfHouses`)))
  (bind _housesarray (`/Game/Assets/Core/BP_WorldManager.PlaceHouses` (`self.WorldManager`) _output_get))
  (set `self.HousesRef` _housesarray)
  (bind _meetpointsarray (`/Game/Assets/Core/BP_WorldManager.PlaceMeetPoints` (`self.WorldManager`) (`self.NumOfMeetPoints`)))
  (set `self.MeetPointsRef` _meetpointsarray)
  (`KismetSystemLibrary.PrintString` "Simulation Starting")
  (`self.HideMenu`)
  (`self.ShowHUD`)
  (set `self.StopSimulation` false)
  (for _array_element (`self.HousesRef`)
    (`/Game/Assets/Blueprints/BP_House.SpawnAgents` _array_element)
    (`/Game/Assets/UI/W_HUD.UpdateAgentsNumberText` _whud _sceptiquesn _croyantsn _ignorantsn)
    (`/Game/Assets/UI/W_HUD.SetGenerationText` _whud _generation)
    (`BlueprintMapLibrary.Map_Add` (`self.Infos`) _generation (make `/Game/Assets/Blueprints/S_GenerationInfos` _sceptiquesn _croyantsn _ignorantsn))
    (set `self.SomeoneNotReady` false :!label _label)
    (bind _returnvalue (`KismetSystemLibrary.K2_SetTimerDelegate` (delegate `CheckForEveryoneReadyToMeeting`) 1.0 true true))))

(event `Resimulate`
  (if (`self.StopSimulation`)
    (`self.CreateResultUI`)
    (else
      (`KismetSystemLibrary.K2_ClearAndInvalidateTimerHandle` (stale `CheckForEveryoneReadyToMeeting` _returnvalue))
      (bind _result (`/Engine/EditorBlueprintResources/StandardMacros.IncrementInt` (`self.Generation`))
        (:`  `
          (`/Game/Assets/UI/W_HUD.SetGenerationText` (`self.WHud`) _result)
          (goto _label))))))

(event `ShowHUD`
  (bind _returnvalue (`|CreateWidget` "/Game/Assets/UI/W_HUD.W_HUD_C"))
  (bind _output_get (set `self.WHud` _returnvalue))
  (`UserWidget.AddToViewport` _output_get 0))

(event `CheckForEveryoneReadyToMeeting`
  (bind (_sceptiquesn _croyantsn _ignorantsn) (`self.CalculateNumbersOfAgentsPerTypes`))
  (set `self.SomeoneNotReady` false)
  (for _array_element (`self.HousesRef`) :!label _label_2
    (for _array_element_2 (`/Game/Assets/Blueprints/BP_House.AgentsRef` _array_element)
      (if (not (`/Game/Assets/Blueprints/AI/BP_AIController.ReadyToMeeting` (`/Game/Assets/Blueprints/AI/BP_Agent.As BP AIController` _array_element_2)))
        (set `self.SomeoneNotReady` true)
        (goto _label_2 :!via `Break`))))
  (if (not (`self.SomeoneNotReady`))
    (`self.StartMeeting`)
    (`/Game/Assets/UI/W_HUD.UpdateAgentsNumberText` (`self.WHud`) _sceptiquesn _croyantsn _ignorantsn)
    (`BlueprintMapLibrary.Map_Add` (`self.Infos`) (`self.Generation`) (make `/Game/Assets/Blueprints/S_GenerationInfos` _sceptiquesn _croyantsn _ignorantsn))
    (`KismetSystemLibrary.PrintString` "MeetingDone")
    (if (`self.StopSimulation`)
      (`self.CreateResultUI`)
      (else
        (set `self.SomeoneNotReady` false)
        (bind _returnvalue (`KismetSystemLibrary.K2_SetTimerDelegate` (delegate `CheckForEveryoneAtHouse`) 1.0 true true))
        (`KismetSystemLibrary.K2_ClearAndInvalidateTimerHandle` (stale `StartSimulation` _returnvalue))))))

(event `CheckForEveryoneAtHouse`
  (set `self.SomeoneNotReady` false)
  (for _array_element (`self.HousesRef`)
    (for _array_element_2 (`/Game/Assets/Blueprints/BP_House.AgentsRef` _array_element)
      (if (`/Game/Assets/Blueprints/AI/BP_AIController.ReadyToMeeting` (`/Game/Assets/Blueprints/AI/BP_Agent.As BP AIController` _array_element_2))
        (set `self.SomeoneNotReady` true))))
  (if (not (`self.SomeoneNotReady`))
    (`self.StartSearchingPoint`)
    (`self.Resimulate`)))

(fn `CalculateNumbersOfAgentsPerTypes`
  (returns (SceptiquesN :type Integer) (CroyantsN :type Integer) (IgnorantsN :type Integer))
  (locals (SceptiquesNum :type Integer) (CroyantsNum :type Integer) (IgnorantsNum :type Integer))
  (set `local.SceptiquesNum` 0)
  (set `local.CroyantsNum` 0)
  (set `local.IgnorantsNum` 0)
  (for _array_element (`self.HousesRef`)
    (for _array_element_2 (`/Game/Assets/Blueprints/BP_House.AgentsRef` _array_element)
      (switch `/Game/Assets/Blueprints/E_AgentState` (`/Game/Assets/Blueprints/AI/BP_Agent.GetState` _array_element_2)
        (:`NewEnumerator0`
          (`/Engine/EditorBlueprintResources/StandardMacros.IncrementInt` (`local.IgnorantsNum`)))
        (:`NewEnumerator1`
          (`/Engine/EditorBlueprintResources/StandardMacros.IncrementInt` (`local.SceptiquesNum`)))
        (:`NewEnumerator2`
          (`/Engine/EditorBlueprintResources/StandardMacros.IncrementInt` (`local.CroyantsNum`))))))
  (return (`local.SceptiquesNum`) (`local.CroyantsNum`) (`local.IgnorantsNum`)))

(fn `CreateResultUI`
  (`/Game/Assets/UI/W_HUD.GenerateResult` (`self.WHud`) (`self.Infos`)))

(fn `DetermineNumberOfHouses`
  (returns (Number :type Integer))
  (bind _returnvalue (/ (`self.NumOfAgents`) 3))
  (if (`self.IsDivisibleBy` (`self.NumOfAgents`) 3)
    (return _returnvalue)
    (else
      (return (+ _returnvalue 1)))))

(fn `HideMenu`
  (`Widget.SetVisibility` (`self.Menu`) "Collapsed")
  (`WidgetBlueprintLibrary.SetInputMode_GameAndUIEx` (`GameplayStatics.GetPlayerController` 0) null "LockAlways" false))

(fn `IsDivisibleBy`
  (params (Value :type Integer) (By :type Integer))
  (returns (Return :type Boolean))
  (return (== (mod Value By) 0)))

(fn `ShowMenu`
  (bind _returnvalue (`GameplayStatics.GetPlayerController` 0))
  (`/Engine/EditorBlueprintResources/StandardMacros.IsValid` (`self.Menu`)
    (:`Is Valid`
      _)
    (:`Is Not Valid`
      (bind _returnvalue_2 (`|CreateWidget` "/Game/Assets/UI/W_Menu.W_Menu_C" (`GameplayStatics.GetPlayerController` 0)))
      (set `self.Menu` _returnvalue_2)))
  (`UserWidget.AddToViewport` (`self.Menu`) 0)
  (set `PlayerController.bShowMouseCursor` true _returnvalue)
  (`WidgetBlueprintLibrary.SetInputMode_UIOnlyEx` _returnvalue (`self.Menu`)))

(fn `StartMeeting`
  (for _array_element (`self.MeetPointsRef`)
    (`/Game/Assets/Blueprints/BP_MeetPoint.UpdateStateOfAgents` _array_element)))

(fn `StartSearchingPoint`
  (for _array_element (`self.HousesRef`)
    (for _array_element_2 (`/Game/Assets/Blueprints/BP_House.AgentsRef` _array_element)
      (`/Game/Assets/Blueprints/AI/BP_AIController.SetMeetingDone` (`/Game/Assets/Blueprints/AI/BP_Agent.As BP AIController` _array_element_2) false))))

(fn `UserConstructionScript`)