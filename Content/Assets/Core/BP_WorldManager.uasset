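; BP_WorldManager lays out the simulation world by spawning houses and meet points around the world origin.
; PlaceHouses spaces BP_House actors evenly on a ring sized from the HouseVolume bounds.
; PlaceMeetPoints spreads BP_MeetPoint actors over a fixed-radius disc using a golden-angle (sunflower) spiral.
; Both functions return the spawned actors for external callers, while BeginPlay only caches the GM_SimulationManager game mode.
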(event `self.ReceiveBeginPlay`
  (bind _asgm_simulation_manager (cast `/Game/Assets/Core/GM_SimulationManager` (`GameplayStatics.GetGameMode`))
    (:`then`
      (set `self.As GM Simulation Manger` _asgm_simulation_manager))
    (:`CastFailed`
      (`KismetSystemLibrary.PrintString` "Error : WorldManager cast to Gamemode failed"))))

(fn `FindRandomPointInCylinder`
  (params (Center :type "Vector Structure") (Radius :type "Float (double-precision)"))
  (locals (GoldenAngle :type "Float (double-precision)")))

(fn `PlaceHouses`
  (params (NumberOfHouses :type Integer))
  (returns (HousesArray :type "Array of /Game/Assets/Blueprints/BP_House Object Reference"))
  (locals (AngleStep :type "Float (double-precision)") (Radius :type "Float (double-precision)") (HousesRef :type "Array of /Game/Assets/Blueprints/BP_House Object Reference"))
  (bind _radius (`local.Radius`))
  (`KismetArrayLibrary.Array_Clear` (`local.HousesRef`))
  (set `local.Radius` (- (.x (`.BoxExtent` (`self.GetActorBounds` (`self.HouseVolume`) false false))) 100.0))
  (set `local.AngleStep` (/ 360 NumberOfHouses))
  (for _index (range NumberOfHouses)
    (bind _returnvalue (* _index (`local.AngleStep`)))
    (bind _returnvalue_2 (`|SpawnActorFromClass` "/Game/Assets/Blueprints/BP_House.BP_House_C" (`KismetMathLibrary.MakeTransform` (`KismetMathLibrary.MakeVector` (* (`KismetMathLibrary.DegCos` _returnvalue) _radius) (* (`KismetMathLibrary.DegSin` _returnvalue) _radius))) "Undefined" "MultiplyWithRoot" null null))
    (`KismetArrayLibrary.Array_Add` (`local.HousesRef`) _returnvalue_2))
  (return (`local.HousesRef`)))

(fn `PlaceMeetPoints`
  (params (NumberOfMeetPoints :type Integer))
  (returns (MeetPointsArray :type "Array of /Game/Assets/Blueprints/BP_MeetPoint Object Reference"))
  (locals (GoldenAngle :type "Float (double-precision)") (Radius :type "Float (double-precision)" :default 0.0) (R :type "Float (double-precision)") (Theta :type "Float (double-precision)") (MeetPoints :type "Array of /Game/Assets/Blueprints/BP_MeetPoint Object Reference"))
  (bind _r (`local.R`))
  (`KismetArrayLibrary.Array_Clear` (`local.MeetPoints`))
  (set `local.Radius` 1200.0)
  (set `local.GoldenAngle` (`KismetMathLibrary.MultiplyByPi` (- 3.0 (`KismetMathLibrary.Sqrt` 5.0))))
  (for _index (range NumberOfMeetPoints)
    (set `local.R` (* (`local.Radius`) (`KismetMathLibrary.Sqrt` (/ _index (`local.NumberOfMeetPoints`)))))
    (bind _output_get (set `local.Theta` (* _index (`local.GoldenAngle`))))
    (bind _returnvalue (`|SpawnActorFromClass` "/Game/Assets/Blueprints/BP_MeetPoint.BP_MeetPoint_C" (`KismetMathLibrary.MakeTransform` (`KismetMathLibrary.MakeVector` (* _r (`KismetMathLibrary.Cos` _output_get)) (* _r (`KismetMathLibrary.Sin` _output_get)))) "AlwaysSpawn" "MultiplyWithRoot" null null))
    (`KismetArrayLibrary.Array_Add` (`local.MeetPoints`) _returnvalue))
  (return (`local.MeetPoints`)))

(fn `UserConstructionScript`)